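; DigitDecoBP is a board decoration actor that shows a single digit from 0 to 9 by swapping the material on its mesh.
; The construction script applies the material for DefaultDigit from the DigitsMats array, so the starting digit is visible in the editor.
; At runtime, the ChangeDigit event range-checks the new value and sets the matching material on slot 0.
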(event `ChangeDigit`
  (params (NewDigit :type Integer))
  (if (and (>= NewDigit 0) (<= NewDigit 9))
    (`PrimitiveComponent.SetMaterial` (`self.Mesh`) 0 (`|GetArrayItem` (`self.DigitsMats`) NewDigit))))

(fn `UserConstructionScript`
  (`parent.UserConstructionScript`)
  (`PrimitiveComponent.SetMaterial` (`self.Mesh`) 0 (`|GetArrayItem` (`self.DigitsMats`) (`self.DefaultDigit`))))